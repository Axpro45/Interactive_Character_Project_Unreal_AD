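; BP_EnemyAI is a melee enemy, counted as a defeated bandit on death, that chases and punches the player.
; PawnSensing sighting triggers AIMoveTo; on arrival it plays a punch montage and damages Player-tagged actors in a sphere overlap at an arrow component.
; Tick halts movement until the player is seen and turns a widget toward the camera.
; Damage drains Health; death increments the player character's KillCount and destroys the enemy.
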(event OnSeePawn(PawnSensing)
  (params (Pawn :type Pawn%20Object%20Reference))
  (Variables|Default|SetIsSeeingPlayer? true)
  (CallFunction|FollowPlayer))

(event Custom|follow%20player
  (Variables|Default|SetCanAttack? true)
  (if (Variables|Default|GetIsSeeingPlayer?)
    (AI|AIMoveTo self "0, 0, 0" (Game|GetPlayerCharacter 0) 7e+01 false
      (:OnSuccess
        (if (Variables|Default|GetCanAttack?)
          (Variables|Default|SetCanAttack? false)
          (bind _returnvalue (Animation|PlayAnimMontage "/Game/Combat/Animations/Retarget_Paired_CounterPunch_PalmStrike_Att_Montage.Retarget_Paired_CounterPunch_PalmStrike_Att_Montage" 1.0 "None"))
          (bind _outactors (Collision|SphereOverlapActors (Transformation|GetWorldLocation (Variables|Default|GetArrow1)) 1e+02 (Variables|Default|GetObject%20Types) 0))
          (bind _array_element (Utilities|Array|ForEachLoopwithBreak _outactors)
            (:LoopBody
              (if (Actor|ActorHasTag _array_element "Player")
                (Game|Damage|ApplyDamage _array_element 5.0 0 0)))
            (:Completed
              (Utilities|FlowControl|Delay _returnvalue)
              (Variables|Default|SetCanAttack? true))))))
    (else
      (Variables|Default|SetIsSeeingPlayer? false))))

(event EventBeginPlay)

(event Collision|EventActorBeginOverlap
  (params (OtherActor :type Actor%20Object%20Reference)))

(event EventTick
  (params (DeltaSeconds :type Float%20%28single-precision%29))
  (Utilities|FlowControl|Sequence
    (:then_0
      (if (not (Variables|Default|GetIsSeeingPlayer?))
        (Components|Movement|StopMovementImmediately (Variables|Character|GetCharacterMovement))))
    (:then_1
      (Transformation|SetWorldRotation (Variables|Default|GetWidget) (Math|Rotator|FindLookatRotation (Transformation|GetWorldLocation (Variables|Default|GetWidget)) (Transformation|GetWorldLocation (Variables|/Script/Engine.PlayerCameraManager|GetTransformComponent (Game|GetPlayerCameraManager 0)))) false false))))

(event Game|Damage|EventAnyDamage
  (params (Damage :type Float%20%28single-precision%29) (DamageType :type Damage%20Type%20Object%20Reference) (InstigatedBy :type Controller%20Object%20Reference) (DamageCauser :type Actor%20Object%20Reference))
  (Variables|Default|SetHealth (- (Variables|Default|GetHealth) Damage))
  (Development|PrintString (Utilities|String|ToString(Float) (Variables|Default|GetHealth)))
  (if (<= (Variables|Default|GetHealth) 0.0)
    ;[1 1 1] Counting kill
    (bind _asbp_third_person_character (Utilities|Casting|CastToBP_ThirdPersonCharacter (Game|Player|GetPlayerPawn 0)))
    (Math|Integer|IncrementInt (Variables|/Game/ThirdPerson/Blueprints/BP_ThirdPersonCharacter.BP_ThirdPersonCharacter_C|GetKillCount _asbp_third_person_character)
      (:%20%20
        (Default|BanditsDeafeated _asbp_third_person_character)
        (Development|PrintString "Kill" true true "(R=1.000000,G=0.000000,B=0.880818,A=1.000000)")
        (Actor|DestroyActor)))))

(fn ConstructionScript)