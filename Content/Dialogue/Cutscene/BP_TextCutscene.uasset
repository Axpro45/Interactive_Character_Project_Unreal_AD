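; BP_TextCutscene is an unfinished text cutscene actor, apparently meant as a typewriter reveal before loading the InteractiveCharacter level.
; DisplayNextLetter re-arms itself by timer every LetterDelay, advancing LetterIndex and setting TextRender to Fulltext, with no substring step shown.
; When its LetterIndex check against Fulltext fails, it opens that level.
; StartCutscene is empty, and the reset and first-call nodes are disconnected, so nothing here starts the loop.
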(event Custom|StartCutscene)

(event EventBeginPlay)

(event Collision|EventActorBeginOverlap
  (params (OtherActor :type Actor%20Object%20Reference)))

(event EventTick
  (params (DeltaSeconds :type Float%20%28single-precision%29)))

(fn ConstructionScript)

(fn DisplayNextLetter
  (if (< (Variables|Default|GetLetterIndex) (Variables|Default|GetFulltext))
    (Variables|Default|SetCurrentText (Variables|Default|GetFulltext))
    (Rendering|Components|TextRender|SetText (Variables|Default|GetTextRender) (Utilities|Text|ToText(String) (Variables|Default|GetCurrentText)))
    (Variables|Default|SetLetterIndex (+ (Variables|Default|GetLetterIndex) 1))
    (Utilities|Time|SetTimerbyFunctionName 0 "DisplayNextLetter" (Variables|Default|GetLetterDelay))
    (else
      (Game|OpenLevel(byName) "InteractiveCharacter "))))