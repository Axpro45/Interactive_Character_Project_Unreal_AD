(event OnComponentEndOverlap(Box)
  (params (OverlappedComponent :type Primitive%20Component%20Object%20Reference) (OtherActor :type Actor%20Object%20Reference) (OtherComp :type Primitive%20Component%20Object%20Reference) (OtherBodyIndex :type Integer))
  ;[1 1 1] changing back to deafult camera view
  (bind _asbp_third_person_character (Utilities|Casting|CastToBP_ThirdPersonCharacter OtherActor))
  (Components|Activation|SetActive (Variables|/Game/ThirdPerson/Blueprints/BP_ThirdPersonCharacter.BP_ThirdPersonCharacter_C|GetFollowCamera _asbp_third_person_character) true false))

(event OnComponentBeginOverlap(Presse)
  (params (OverlappedComponent :type Primitive%20Component%20Object%20Reference) (OtherActor :type Actor%20Object%20Reference) (OtherComp :type Primitive%20Component%20Object%20Reference) (OtherBodyIndex :type Integer) (bFromSweep :type Boolean) (SweepResult :type Hit%20Result%20Structure%20%28by%20ref%29))
  ;[1 1 1] Press e to interact
)

(event Custom|newdialogue
  ;[1 1 1] enemies deafeted dialogue
  (bind _returnvalue (UserInterface|CreateWidget "/Game/Dialogue/WB_thankyou1.WB_thankyou1_C" (Game|GetPlayerController 0)))
  (Variables|Default|SetUI 0)
  (UserInterface|Viewport|AddtoViewport _returnvalue 0)
  (Widget|RemovefromParent (Variables|Default|GetUI))
  (Utilities|FlowControl|Delay 1e+01)
  (UserInterface|CreateWidget "/Game/Dialogue/Cutscene/WB_Outro.WB_Outro_C" (Game|GetPlayerController 0)))

(event EventTalk
  (bind _returnvalue (Game|GetPlayerController 0))
  ;[1 1 1] enemies deafeted dialogue
  (bind _returnvalue_2 (Actor|GetActorOfClass "/Game/ThirdPerson/Blueprints/BP_ThirdPersonCharacter.BP_ThirdPersonCharacter_C"))
  (Pawn|Components|CharacterMovement|DisableMovement (Variables|/Script/Engine.Character|GetCharacterMovement _returnvalue_2))
  (if (== (Variables|/Game/ThirdPerson/Blueprints/BP_ThirdPersonCharacter.BP_ThirdPersonCharacter_C|GetKillCount _returnvalue_2) 2)
    (Default|BanditsDeafeated _returnvalue_2)
    (CallFunction|Newdialogue)
    (elif (>= (Variables|Default|Gettalkindex) 4)
      (if (Variables|Default|GetDecision)
        (bind _result (Math|Integer|IncrementInt (Variables|Default|Gettalkindex) :!label _label)
          (:%20%20
            ;[0 0 1] Print to track the progress
            (Development|PrintString (Utilities|String|ToString(Integer) _result))
            (switch int (Variables|Default|Gettalkindex)
              (:0
                (Variables|Default|GetUI :!label _label_2
                  (:then
                    (UserInterface|Viewport|AddtoViewport (Variables|Default|GetUI) 0))
                  (:else
                    (Development|PrintString "is not valid")
                    (bind _returnvalue_3 (UserInterface|CreateWidget "/Game/Dialogue/WB_Dialogue.WB_Dialogue_C" (Game|GetPlayerController 0)))
                    (bind _output_get (Variables|Default|SetUI _returnvalue_3))
                    (UserInterface|Viewport|AddtoViewport _output_get 0)))
                (Rendering|Components|TextRender|SetText (Variables|/Game/Dialogue/WB_Dialogue.WB_Dialogue_C|GetTalk_Dialogue (Variables|Default|GetUI)) (Utilities|Text|ToText(String) (Utilities|Array|Get(acopy) (Variables|Default|GetDialogue) (Variables|Default|Gettalkindex)))))
              (:1
                (goto _label_2))
              (:2
                (goto _label_2))
              (:3
                (goto _label_2))
              (:4
                ;[1 1 1] Button stuff
                (if (Variables|Default|GetAccepted)
                  (Variables|Default|Settalkindex 0)
                  (else
                    (Widget|RemovefromParent _returnvalue_3)
                    (bind _returnvalue_4 (UserInterface|CreateWidget "/Game/Dialogue/WB_Willyouhelp.WB_Willyouhelp_C" (Game|GetPlayerController 0)))
                    (UserInterface|Viewport|AddtoViewport _returnvalue_4 0)
                    (Variables|/Script/Engine.PlayerController|SetbShowMouseCursor (Game|GetPlayerController 0) true)
                    (if (Variables|Default|GetAccepted)
                      (Widget|RemovefromParent (Variables|Default|GetUI))
                      (Development|PrintString "Accepted")
                      (bind _returnvalue_5 (UserInterface|CreateWidget "/Game/Dialogue/WB_Dialogue.WB_Dialogue_C" (Game|GetPlayerController 0)))
                      (UserInterface|Viewport|AddtoViewport _returnvalue_5 0)
                      (Variables|/Script/Engine.PlayerController|SetbShowMouseCursor (Game|GetPlayerController 0) false)
                      (Variables|Default|Settalkindex 5)))))
              (:5
                (if (Variables|Default|GetDecision) :!label _label_3
                  (goto _label_2)))
              (:6
                (goto _label_3))
              (:7
                ;[1 1 1] finish talking
                (bind _returnvalue_6 (Actor|GetActorOfClass "/Game/ThirdPerson/Blueprints/BP_ThirdPersonCharacter.BP_ThirdPersonCharacter_C"))
                (Components|Activation|SetActive (Variables|/Game/ThirdPerson/Blueprints/BP_ThirdPersonCharacter.BP_ThirdPersonCharacter_C|GetCutscene%20cam _returnvalue_6) false false)
                (Components|Activation|SetActive (Variables|/Game/ThirdPerson/Blueprints/BP_ThirdPersonCharacter.BP_ThirdPersonCharacter_C|GetFollowCamera _returnvalue_6) true false)
                (Default|EnableInput _returnvalue_6)
                (Widget|RemovefromParent (Variables|Default|GetUI))
                ;[1 1 1] putting healthbar back on after widget removes it
                (bind _returnvalue_7 (UserInterface|CreateWidget "/Game/Health/WP_HealthBar.WP_HealthBar_C" _returnvalue))
                (UserInterface|Viewport|AddtoViewport _returnvalue_7 0)
                (Input|SetInputModeGameOnly _returnvalue false)
                (Pawn|Components|CharacterMovement|SetMovementMode (Variables|/Script/Engine.Character|GetCharacterMovement _returnvalue_6) "MOVE_Walking" 0)
                ;[1 1 1] Trying to get new widget update to spawn
                (bind _returnvalue_8 (UserInterface|CreateWidget "/Game/Dialogue/WB_questtracker.WB_questtracker_C" _returnvalue))
                (UserInterface|Viewport|AddtoViewport _returnvalue_8 0)
                (bind _returnvalue_9 (Actor|GetActorOfClass "/Game/ThirdPerson/Blueprints/BP_ThirdPersonCharacter.BP_ThirdPersonCharacter_C"))
                (if (== (Math|Conversions|ToBoolean(Integer) (Variables|/Game/ThirdPerson/Blueprints/BP_ThirdPersonCharacter.BP_ThirdPersonCharacter_C|GetKillCount _returnvalue_9)) 2)
                  (Widget|RemovefromParent _returnvalue_8)))))))
      (else
        (goto _label)))))

(fn ConstructionScript)